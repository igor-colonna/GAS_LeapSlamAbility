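; Leap slam gameplay ability that jumps the character to the navmesh-projected point under the mouse and damages nearby pawns.
; Out-of-range targets trigger a cancelable auto-run into range first.
; The leap plays a montage, teleports the capsule using the arc result and moves the mesh along a spline, realigning both afterward or on cancel.
; A montage event spawns ground-breaking VFX and sphere-traces for damage; an ongoing effect lasts until the ability ends.
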(event `self.K2_ActivateAbility`
  (bind _gascharacter (`self.GASCharacter`))
  (bind _projected_location (`self.Projected Location`))
  (bind _mesh (`Character.Mesh` _gascharacter))
  (bind _capsulecomponent (`Character.CapsuleComponent` _gascharacter))
  ;[0.09168 0.2511 0.849 0.5] Target Location Aquisition
  (bind (_asynctaskproxy _datahandle) (`TargetDataUnderMouse.CreateTargetDataUnderMouse`)
    (:`ValidData`
      (bind (_projectedlocation _returnvalue) (`NavigationSystemV1.K2_ProjectPointToNavigation` (`.ImpactPoint` (`GameplayStatics.BreakHitResult` (`AbilitySystemBlueprintLibrary.GetHitResultFromTargetData` _datahandle)))))
      (bind _output_get (set `self.Projected Location` _projectedlocation))
      (if (> (`KismetMathLibrary.Distance2D` (`KismetMathLibrary.Conv_VectorToVector2D` (`Actor.K2_GetActorLocation` (`self.GASCharacter`))) (`KismetMathLibrary.Conv_VectorToVector2D` _output_get)) (`self.AbilityRange`))
        ;[0.9635 0.08531 0.08531 0.5] Handle Out of Range
        (`self.SetCanBeCanceled` true)
        (bind (_branches _outlocation _outpath) (`self.CalculatePointWithinRange` (`Actor.K2_GetActorLocation` (`self.GASCharacter`)) (`self.Projected Location`)))
        (switch `ECalculatePointResult` _branches
          (:`Invalid`
            (`KismetSystemLibrary.PrintString` "Invalid Path")
            (`self.K2_EndAbility`))
          (:`Valid`
            (`GAS_AutoRun.CreateAutoRunTask` _outlocation (`self.SplineComp`) _outpath 50.0 true
              (:`OnCompleted`
                (set `self.LookRotation` (`KismetMathLibrary.FindLookAtRotation` (`Actor.K2_GetActorLocation` (`self.GASCharacter`)) (`self.Projected Location`)) :!label _label)
                (`self.SetCanBeCanceled` false)
                (bind _returnvalue_2 (`self.BP_ApplyGameplayEffectToOwner` "/Game/Hexborne_Test/AbilitySystem/GameplayEffects/GE_AddLeapSlamOngoing.GE_AddLeapSlamOngoing_C"))
                (set `self.BlockedAbilitiesSpecHandle` _returnvalue_2)
                (`AbilityTask_PlayMontageAndWait.CreatePlayMontageAndWaitProxy` "None" "/Game/Hexborne_Test/Character/Anims/AM_LeapSlam2.AM_LeapSlam2"
                  (:`then`
                    (if _returnvalue
                      ;[0.07301 0.9323 0.1361 0.5] Getting the arc to target location
                      (bind _outend (`self.CreateArc` (`Actor.K2_GetActorLocation` (`self.GASCharacter`)) (`self.Projected Location`) 100.0))
                      (`SceneComponent.K2_SetWorldLocationAndRotation` _capsulecomponent (`KismetMathLibrary.MakeVector` (.x _outend) (.y _outend) (+ (.z _outend) (`CapsuleComponent.CapsuleHalfHeight` _capsulecomponent))) (`self.LookRotation`) false true)
                      (bind (_asynctaskproxy_2 _movefinished) (`GameplayTask_MoveAlongSpline.CreateMoveAlongSplineTask` _mesh (`self.SplineComp`) 1.0)
                        (:`then`
                          (`AbilityTask_WaitGameplayEvent.WaitGameplayEvent` (struct :`TagName` "Event.Montage.LeapSlamHit") null
                            (:`EventReceived`
                              (`NiagaraFunctionLibrary.SpawnSystemAtLocation` "/Game/Hexborne_Test/FX/NS_GroundBreaking.NS_GroundBreaking" (`self.Projected Location`))
                              ;[1 0.01872 0 0.5] Damage causing logic
                              (bind _outhits (`KismetSystemLibrary.SphereTraceMultiForObjects` _projected_location _projected_location 200.0 (`|MakeArray` "ObjectTypeQuery3" :!type "EObjectTypeQuery Enum") false (`|MakeArray` (`self.GetAvatarActorFromActorInfo`)) "ForDuration"))
                              (for _array_element _outhits
                                (`self.BP_ApplyGameplayEffectToTarget` (`AbilitySystemBlueprintLibrary.AbilityTargetDataFromActor` (`.HitActor` (`GameplayStatics.BreakHitResult` _array_element))) "/Game/Hexborne_Test/AbilitySystem/GameplayEffects/Damage/GE_Damage.GE_Damage_C" (`self.GetAbilityLevel`))))))
                        (:`OnMoveFinished`
                          (`self.Correct Capsule/Mesh Location` _capsulecomponent _mesh true)))
                      (else
                        (`self.K2_EndAbility`))))
                  (:`OnCompleted`
                    (if _movefinished
                      (`self.K2_EndAbility`)))
                  (:`OnInterrupted`
                    (`self.K2_CancelAbility` :!label _label_2))
                  (:`OnCancelled`
                    (goto _label_2)))))))
        (else
          (goto _label))))))

(event `self.K2_OnEndAbility`
  (params (bWasCancelled :type Boolean))
  (bind _gascharacter (`self.GASCharacter`))
  (if bWasCancelled
    (`KismetSystemLibrary.PrintString` "Ability Cancelled")
    (`self.Correct Capsule/Mesh Location` (`Character.CapsuleComponent` _gascharacter) (`Character.Mesh` _gascharacter))
    (else
      (`KismetSystemLibrary.PrintString` "Ability Ended")))
  (`self.BP_RemoveGameplayEffectFromOwnerWithHandle` (`self.BlockedAbilitiesSpecHandle`)))

(fn `Correct Capsule/Mesh Location`
  (params (CapusleComponent :type "SceneComponent Object Reference") (`Mesh Component` :type "SceneComponent Object Reference") (`MeshToCapsule?` :type Boolean))
  (bind (_returnvalue_x _returnvalue_y _returnvalue_z) (`KismetMathLibrary.BreakVector` (`SceneComponent.K2_GetComponentLocation` `Mesh Component`)))
  (bind (_returnvalue_x_2 _returnvalue_y_2 _returnvalue_z_2) (`KismetMathLibrary.BreakVector` (`SceneComponent.K2_GetComponentLocation` CapusleComponent)))
  (if (not `MeshToCapsule?`)
    (`SceneComponent.K2_SetWorldLocation` CapusleComponent (`KismetMathLibrary.MakeVector` _returnvalue_x _returnvalue_y _returnvalue_z) false true))
  (`SceneComponent.K2_SetWorldLocation` `Mesh Component` (`KismetMathLibrary.MakeVector` _returnvalue_x_2 _returnvalue_y_2 (- _returnvalue_z_2 100.0)) false true))